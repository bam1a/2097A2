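; End-game pickup actor that explodes and declares a match winner when hit by a ThirdPersonCharacter holding a named pickup.
; The mesh hit handler calls EmitExplosion, whose body is outside this graph.
; EmitExplosionBP, on authority only, sets "Server" as winner in the game mode, while clientEmitExplosion sets "Client" without an authority switch.
; Both events then share one chain that spawns explosion particles and sound and destroys the actor.
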(event OnComponentHit(StaticMeshComponent)
  (params (HitComponent :type Primitive%20Component%20Object%20Reference) (OtherActor :type Actor%20Object%20Reference) (OtherComp :type Primitive%20Component%20Object%20Reference) (NormalImpulse :type Vector :default "0, 0, 0") (Hit :type Hit%20Result%20Structure%20%28by%20ref%29))
  (bind _ascharacter (Utilities|Casting|CastToCharacter OtherActor))
  (bind _asthird_person_character (Utilities|Casting|CastToThirdPersonCharacter _ascharacter))
  (if (Utilities|Enum|NotEqual(Enum) (Variables|/Script/MyProject.MyProjectCharacter|GetPickupName _asthird_person_character) "")
    (Class|EmitPickup|EmitExplosion)))

(event Custom|client%20Emit%20Explosion
  (bind _staticmeshcomponent (Variables|Default|GetStaticMeshComponent))
  (bind _returnvalue (Transformation|GetWorldLocation _staticmeshcomponent))
  ;[1 1 1] before explosion, claim the winner to the game mode first
  (bind _asmy_my_project_game_mode (Utilities|Casting|CastToMyMyProjectGameMode (Game|GetGameMode)))
  (Class|MyProjectGameMode|SetWinner _asmy_my_project_game_mode "Client")
  (Effects|SpawnEmitteratLocation "/Game/StarterContent/Particles/P_Explosion.P_Explosion" _returnvalue)
  (Audio|PlaySoundatLocation "/Game/StarterContent/Audio/Explosion_Cue.Explosion_Cue" _returnvalue "0, 0, 0" 1.0 1.0 0.0 0 0 0)
  (Actor|DestroyActor))

(event EventBeginPlay)

(event Collision|EventActorBeginOverlap
  (params (OtherActor :type Actor%20Object%20Reference)))

(event EventTick
  (params (DeltaSeconds :type Float%20%28single-precision%29)))

(event EventEmitExplosionBP
  (bind _staticmeshcomponent (Variables|Default|GetStaticMeshComponent))
  (bind _returnvalue (Transformation|GetWorldLocation _staticmeshcomponent))
  ;[1 1 1] before explosion, claim the winner to the game mode first
  (Networking|SwitchHasAuthority
    (:Authority
      (bind _asmy_my_project_game_mode (Utilities|Casting|CastToMyMyProjectGameMode (Game|GetGameMode)))
      (Class|MyProjectGameMode|SetWinner _asmy_my_project_game_mode "Server")
      (Effects|SpawnEmitteratLocation "/Game/StarterContent/Particles/P_Explosion.P_Explosion" _returnvalue)
      (Audio|PlaySoundatLocation "/Game/StarterContent/Audio/Explosion_Cue.Explosion_Cue" _returnvalue "0, 0, 0" 1.0 1.0 0.0 0 0 0)
      (Actor|DestroyActor))))

(fn ConstructionScript)