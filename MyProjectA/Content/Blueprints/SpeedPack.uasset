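; SpeedPack is a pickup that boosts the third-person character's speed when hit, provided the character's PickupName matches its own.
; The static mesh's hit event casts to ThirdPersonCharacter, calls AddSpeedMultiplier with a fixed amount, then calls EmitExplosion.
; A separate EmitExplosionBP event spawns the explosion particles and sound at the mesh and destroys the actor.
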(event OnComponentHit(StaticMeshComponent)
  (params (HitComponent :type Primitive%20Component%20Object%20Reference) (OtherActor :type Actor%20Object%20Reference) (OtherComp :type Primitive%20Component%20Object%20Reference) (NormalImpulse :type Vector :default "0, 0, 0") (Hit :type Hit%20Result%20Structure%20%28by%20ref%29))
  ;[1 1 1] make sure the actor is the character hits
  (bind _asthird_person_character (Utilities|Casting|CastToThirdPersonCharacter OtherActor))
  (if (Utilities|Enum|Equal(Enum) (Variables|/Script/MyProject.MyProjectCharacter|GetPickupName _asthird_person_character) (Variables|Default|GetpickupName))
    (Class|MyProjectCharacter|AddSpeedMultiplier _asthird_person_character 3e+01)
    (Class|EmitPickup|EmitExplosion)))

(event EventBeginPlay)

(event Collision|EventActorBeginOverlap
  (params (OtherActor :type Actor%20Object%20Reference)))

(event EventTick
  (params (DeltaSeconds :type Float%20%28single-precision%29)))

(event EventEmitExplosionBP
  (bind _staticmeshcomponent (Variables|Default|GetStaticMeshComponent))
  (bind _returnvalue (Transformation|GetWorldLocation _staticmeshcomponent))
  (Effects|SpawnEmitteratLocation "/Game/StarterContent/Particles/P_Explosion.P_Explosion" _returnvalue)
  (Audio|PlaySoundatLocation "/Game/StarterContent/Audio/Explosion_Cue.Explosion_Cue" _returnvalue "0, 0, 0" 1.0 1.0 0.0 0 0 0)
  (Actor|DestroyActor))

(fn ConstructionScript)