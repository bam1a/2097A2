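; Game mode Blueprint that shows the end-of-match result screen when there is a winner or when all players lose.
; HasWinnerBP and AllLoserBP each call a matching multicast-named event, which creates the WinnerHUD or LoserHUD widget and adds it to the viewport.
; A StringCall helper prints a given string as text, while BeginPlay, Tick and the construction script are empty.
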(event Custom|has%20winner%20multicast
  (bind _returnvalue (UserInterface|CreateWidget "/Game/HUD/winnerHUD.winnerHUD_C"))
  (UserInterface|Viewport|AddtoViewport _returnvalue 0))

(event Custom|all%20loser%20multicast
  (bind _returnvalue (UserInterface|CreateWidget "/Game/HUD/loserHUD.loserHUD_C"))
  (UserInterface|Viewport|AddtoViewport _returnvalue 0))

(event EventBeginPlay)

(event EventTick
  (params (DeltaSeconds :type Float%20%28single-precision%29)))

(event EventHasWinnerBP
  (CallFunction|HasWinnerMulticast))

(event EventAllLoserBP
  (CallFunction|AllLoserMulticast))

(fn ConstructionScript)

(fn StringCall
  (params (inString :type String))
  (Development|PrintText (Utilities|Text|ToText(String) inString)))