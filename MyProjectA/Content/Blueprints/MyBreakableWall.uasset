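; A breakable wall actor that loses health when its mesh is hit, then explodes with an emitter and collapse sound and destroys itself.
; Hits route by authority through client, server and multicast events, subtracting player 0's hit power scaled by frame delta.
; Render updates set the material's "emit power" from the health ratio, copy health into a name string and trigger the break at zero.
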(event OnComponentHit(StaticMeshComponent)
  (params (HitComponent :type Primitive%20Component%20Object%20Reference) (OtherActor :type Actor%20Object%20Reference) (OtherComp :type Primitive%20Component%20Object%20Reference) (NormalImpulse :type Vector :default "0, 0, 0") (Hit :type Hit%20Result%20Structure%20%28by%20ref%29))
  (Class|BreakableWall|OnHit))

(event Custom|onHitMulticast
  (bind _asthird_person_character (Utilities|Casting|CastToThirdPersonCharacter (Game|GetPlayerCharacter 0)))
  (Variables|Default|SetwHP (- (Variables|Default|GetwHP) (* (Utilities|Time|GetWorldDeltaSeconds) (Class|MyProjectCharacter|GetHitPower _asthird_person_character))))
  (Class|BreakableWall|UpdateWallRender))

(event Custom|onHitClient
  (CallFunction|OnHitServer))

(event Custom|onHitServer
  (CallFunction|OnHitMulticast))

(event EventBeginPlay)

(event Collision|EventActorBeginOverlap
  (params (OtherActor :type Actor%20Object%20Reference)))

(event EventTick
  (params (DeltaSeconds :type Float%20%28single-precision%29)))

(event EventUpdateWallRenderBP
  (bind _whp (Variables|Default|GetwHP))
  (Rendering|Material|SetScalarParameterValueonMaterials (Variables|Default|GetStaticMeshComponent) "emit power" (/ _whp (Variables|Default|GettopHP)))
  (Variables|Default|SetwName (Utilities|String|ToString(Float) _whp))
  (if (<= _whp 0.0)
    (Class|BreakableWall|WallBreak)))

(event EventWallBreakBP
  (bind _arrow (Variables|Default|GetArrow))
  (bind _returnvalue (Transformation|GetWorldLocation _arrow))
  (Effects|SpawnEmitteratLocation "/Game/StarterContent/Particles/P_Explosion.P_Explosion" _returnvalue "0.000000, 0, 0" "5.000000,5.000000,5.000000")
  (Audio|PlaySoundatLocation "/Game/StarterContent/Audio/Collapse_Cue.Collapse_Cue" _returnvalue "0, 0, 0" 1.0 1.0 0.0 0 0 0)
  (Actor|DestroyActor))

(event EventOnHitBP
  (Networking|SwitchHasAuthority
    (:Authority
      (CallFunction|OnHitMulticast))
    (:Remote
      (CallFunction|OnHitClient))))

(fn ConstructionScript)

(fn HitAAA)