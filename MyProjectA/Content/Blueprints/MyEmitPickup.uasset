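; MyEmitPickup is an actor that explodes when hit by a third-person character carrying a named pickup.
; Its static mesh hit event casts to ThirdPersonCharacter and calls EmitExplosion if PickupName is non-empty.
; A separate EmitExplosionBP event spawns the explosion particle at the mesh location and destroys the actor.
; EmitExplosion is not defined in this graph, so its link to that event lies outside it.
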(event OnComponentHit(StaticMeshComponent)
  (params (HitComponent :type Primitive%20Component%20Object%20Reference) (OtherActor :type Actor%20Object%20Reference) (OtherComp :type Primitive%20Component%20Object%20Reference) (NormalImpulse :type Vector :default "0, 0, 0") (Hit :type Hit%20Result%20Structure%20%28by%20ref%29))
  (bind _ascharacter (Utilities|Casting|CastToCharacter OtherActor))
  (bind _asthird_person_character (Utilities|Casting|CastToThirdPersonCharacter _ascharacter))
  (if (Utilities|Enum|NotEqual(Enum) (Variables|/Script/MyProject.MyProjectCharacter|GetPickupName _asthird_person_character) "")
    (Class|EmitPickup|EmitExplosion)))

(event EventBeginPlay)

(event Collision|EventActorBeginOverlap
  (params (OtherActor :type Actor%20Object%20Reference)))

(event EventTick
  (params (DeltaSeconds :type Float%20%28single-precision%29)))

(event EventEmitExplosionBP
  (Effects|SpawnEmitteratLocation "/Game/StarterContent/Particles/P_Explosion.P_Explosion" (Transformation|GetWorldLocation (Variables|Default|GetStaticMeshComponent)))
  (Actor|DestroyActor))

(fn ConstructionScript)